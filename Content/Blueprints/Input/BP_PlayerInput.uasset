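; BP_PlayerInput handles mouse selection on the hex-tile board, showing the cursor on BeginPlay.
; A left click traces the Visibility channel under the cursor and identifies a HexTile or Unit.
; The tile's index or the unit's current coordinate goes to InputConnectListener along with a GameplayManager.
; That manager comes from an empty loop over all GameplayManager actors at BeginPlay, read later through the loop's element pin.
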(event EventBeginPlay
  (Variables|Default|SetbShowMouseCursor true)
  (bind _outactors (Actor|GetAllActorsOfClass "/Script/heksy.GameplayManager"))
  (for _array_element _outactors
    _))

(event EventTick
  (params (DeltaSeconds :type Float%20%28single-precision%29)))

(event Input|MouseEvents|LeftMouseButton
  (params (Key :type Key%20Structure :default "None"))
  (bind _returnvalue (Game|GetPlayerController 0))
  (bind _hitresult (Game|Player|GetHitResultUnderCursorbyChannel _returnvalue "TraceTypeQuery1" true))
  (bind (_bblockinghit _binitialoverlap _time _distance _location _impactpoint _normal _impactnormal _physmat _hitactor) (Collision|BreakHitResult _hitresult))
  (:Pressed
    (if _bblockinghit
      (bind _ashex_tile (Utilities|Casting|CastToHexTile _hitactor)
        (:then
          (Class|ReadWriteFile|InputConnectListener (Variables|/Script/heksy.HexTile|GetTileIndex _ashex_tile) (stale EventBeginPlay _array_element)))
        (:CastFailed
          (bind _asunit (Utilities|Casting|CastToUnit _hitactor))
          (Class|ReadWriteFile|InputConnectListener (Variables|/Script/heksy.Unit|GetCurrentCord _asunit) (stale EventBeginPlay _array_element)))))))

(fn ConstructionScript)